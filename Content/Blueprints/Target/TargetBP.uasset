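; TargetBP is a shootable-style target actor that takes damage, awards score to whoever hits it, and is destroyed when its health runs out.
; On BeginPlay it applies a dynamic material instance and registers with the game mode.
; Each hit sends its score to the hitter, reduces health and lerps the material color from green toward red by remaining health.
; At zero health it notifies the game mode of its removal before destroying itself.
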(event `self.ReceiveBeginPlay`
  (set `self.StartHealth` (`self.TargetHealth`))
  (bind _returnvalue (`KismetMaterialLibrary.CreateDynamicMaterialInstance` "/Game/Materials/TargetMat.TargetMat"))
  (bind _output_get (set `self.DynamicMat` _returnvalue))
  (`PrimitiveComponent.SetMaterial` (`self.Target`) 0 _output_get)
  (`self.SetColor`)
  (message `/Game/Blueprints/GameModeBPI.AddTarget` (`GameplayStatics.GetGameMode`)))

(event `/Game/Blueprints/Target/TargetBPI.HandleTargetHit`
  (params (Hitter :type "Actor Object Reference") (DamageValue :type Integer))
  (message `/Game/Blueprints/Character/FPSControllerBPI.HandleScoreUpdate` Hitter (`self.TargetScore`))
  (bind _output_get (set `self.TargetHealth` (- (`self.TargetHealth`) DamageValue)))
  (`self.SetColor`)
  (if (<= _output_get 0)
    (message `/Game/Blueprints/GameModeBPI.RemoveTarget` (`GameplayStatics.GetGameMode`))
    (`self.K2_DestroyActor`)))

(fn `SetColor`
  (`MaterialInstanceDynamic.SetVectorParameterValue` (`self.DynamicMat`) "Color" (`KismetMathLibrary.LinearColorLerp` (struct :`R` 1.0 :`A` 1.0) (struct :`G` 1.0 :`A` 1.0) (/ (`KismetMathLibrary.Conv_IntToDouble` (`self.TargetHealth`)) (`KismetMathLibrary.Conv_IntToDouble` (`self.StartHealth`))))))

(fn `UserConstructionScript`)