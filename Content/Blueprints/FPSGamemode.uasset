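; FPS game mode that tracks remaining targets and ends the game when none are left.
; AddTarget and RemoveTarget events adjust TargetRemaining, and RemoveTarget calls GameOver once the count reaches zero or below.
; BeginPlay runs GameStart to set game-only input with a hidden cursor.
; GameOver shows the GameOverHUD widget, switches to UI-only input and reveals the cursor.
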(event `/Game/Blueprints/GameModeBPI.AddTarget`
  (set `self.TargetRemaining` (+ (`self.TargetRemaining`) 1)))

(event `/Game/Blueprints/GameModeBPI.RemoveTarget`
  (bind _output_get (set `self.TargetRemaining` (- (`self.TargetRemaining`) 1)))
  (if (<= _output_get 0)
    (`self.GameOver`)))

(event `self.ReceiveBeginPlay`
  (`self.GameStart`))

(fn `GameOver`
  (bind _returnvalue (`GameplayStatics.GetPlayerController` 0))
  (bind _returnvalue_2 (`|CreateWidget` "/Game/UI/GameOverHUD.GameOverHUD_C"))
  (`UserWidget.AddToViewport` _returnvalue_2 0)
  (`WidgetBlueprintLibrary.SetInputMode_UIOnlyEx` _returnvalue)
  (set `PlayerController.bShowMouseCursor` true _returnvalue))

(fn `GameStart`
  (bind _returnvalue (`GameplayStatics.GetPlayerController` 0))
  (`WidgetBlueprintLibrary.SetInputMode_GameOnly` _returnvalue)
  (set `PlayerController.bShowMouseCursor` false _returnvalue))

(fn `UserConstructionScript`)