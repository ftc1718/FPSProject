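; First-person player character with stamina-limited sprinting, crouch, jump, crosshair HUD and hitscan firing.
; Sprint toggles walk speed and self-rescheduling timers that drain or regenerate stamina, dropping to walk speed when exhausted.
; Stamina changes are sent to the controller for display updates.
; Firing line-traces from the camera, spawns impact particles and sends damage with the controller as hitter to TargetBPI actors.
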(event `DecreaseStamina`
  ;[1 1 1] 有体力的奔跑
  (bind _output_get (set `self.CurrentStamina` (- (`self.CurrentStamina`) (`self.StaminaRate`))))
  (if (< _output_get 0)
    (set `CharacterMovementComponent.MaxWalkSpeed` (`self.WalkSpeed`) (`self.CharacterMovement`))
    (else
      (`KismetSystemLibrary.K2_SetTimer` null "DecreaseStamina" 0.5)
      (message `/Game/Blueprints/Character/FPSControllerBPI.HandleStaminaUpdate` (`self.GetController`) (`self.CurrentStamina`)))))

(event `IncreaseStamina`
  ;[1 1 1] 有体力的奔跑
  (bind _output_get (set `self.CurrentStamina` (+ (`self.CurrentStamina`) (`self.StaminaRate`))))
  (if (<= _output_get (`self.Stamina`))
    (`KismetSystemLibrary.K2_SetTimer` null "IncreaseStamina" 0.5)
    (message `/Game/Blueprints/Character/FPSControllerBPI.HandleStaminaUpdate` (`self.GetController`) (`self.CurrentStamina`))
    (else
      (set `self.CurrentStamina` (`self.Stamina`)))))

(event `/Game/Blueprints/Character/FPSBPI.ToggelSprint`
  (params (IsSprint :type Boolean))
  ;[1 1 1] 有体力的奔跑
  (if IsSprint
    (`KismetSystemLibrary.K2_ClearTimer` null "IncreaseStamina")
    (`KismetSystemLibrary.K2_SetTimer` null "DecreaseStamina" 0.5)
    (set `CharacterMovementComponent.MaxWalkSpeed` (`self.SprintSpeed`) (`self.CharacterMovement`))
    (else
      (`KismetSystemLibrary.K2_ClearTimer` null "DecreaseStamina")
      (`KismetSystemLibrary.K2_SetTimer` null "IncreaseStamina" 0.5)
      (set `CharacterMovementComponent.MaxWalkSpeed` (`self.WalkSpeed`) (`self.CharacterMovement`)))))

(event `/Game/Blueprints/Character/FPSBPI.ToggleCrouch`
  (params (IsCrouched :type Boolean))
  (if IsCrouched
    (`self.Crouch`)
    (else
      (`self.UnCrouch`))))

(event `self.ReceiveBeginPlay`
  ;[1 1 1] Crosshair HUD
  (`self.CreateHUD`)
  (message `/Game/Blueprints/Character/FPSControllerBPI.HandleStaminaUpdate` (`self.GetController`) (`self.Stamina`)))

(event `/Game/Blueprints/Character/FPSBPI.ToggleJump`
  (`self.Jump`))

(event `/Game/Blueprints/Character/FPSBPI.HandleFire`
  (bind _fpscamera (`self.FPSCamera`))
  (bind _returnvalue (`SceneComponent.K2_GetComponentLocation` _fpscamera))
  ;[1 1 1] 射线追踪
  (bind (_outhit _returnvalue_2) (`KismetSystemLibrary.LineTraceSingle` _returnvalue (+ _returnvalue (* (`KismetMathLibrary.GetForwardVector` (`SceneComponent.K2_GetComponentRotation` _fpscamera)) 1000.0)) "TraceTypeQuery1"))
  (if _returnvalue_2
    (bind (_bblockinghit _binitialoverlap _time _location _impactpoint _normal _impactnormal _physmat _hitactor) (`GameplayStatics.BreakHitResult` _outhit))
    (`GameplayStatics.SpawnEmitterAtLocation` "/Game/Particle/HitParticle.HitParticle" _location)
    (if (`KismetSystemLibrary.DoesImplementInterface` _hitactor "/Game/Blueprints/Target/TargetBPI.TargetBPI_C")
      ;[1 1 1] 左下角的目标表明调用该事件的对象
      (message `/Game/Blueprints/Target/TargetBPI.HandleTargetHit` _hitactor (`self.GetController`) (`self.DamageValue`)))))

(fn `CreateHUD`
  (bind _returnvalue (`|CreateWidget` "/Game/UI/Crosshair.Crosshair_C"))
  (`UserWidget.AddToViewport` _returnvalue 0))

(fn `UserConstructionScript`
  (set `self.CurrentStamina` (`self.Stamina`))
  (set `CharacterMovementComponent.MaxWalkSpeed` (`self.WalkSpeed`) (`self.CharacterMovement`)))