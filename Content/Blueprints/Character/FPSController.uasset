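; First-person player controller that handles input and owns the player's score and HUD, so the score survives character death.
; Sprint, crouch, jump and fire go to the controlled pawn through interface messages rather than casts, while look and yaw-based movement are applied directly.
; Held fire repeats via a gate and a 0.2-second retriggerable delay.
; Score and stamina update events refresh ScoreHUD, and GetScore exposes the total.
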(event `self.ReceiveBeginPlay`
  ;[1 1 1] 分数记录在Controller中防止由于角色死亡而丢失
  (`self.CreateScoreHUD`)
  (`self.ScoreUpdate` (`self.PlayerScore`)))

(event `/Game/Blueprints/Character/FPSControllerBPI.HandleScoreUpdate`
  (params (ScorePoint :type Integer))
  ;[1 1 1] 使用接口可以避免当调用函数的Actor被删除时出现的错误（当使用接口时若调用该函数的Actor被删除该接口不产生作用）
  (`self.ScoreUpdate` ScorePoint))

(event `/Game/Blueprints/Character/FPSControllerBPI.HandleStaminaUpdate`
  (params (Stamina :type Integer))
  (`self.StaminaUpdate` Stamina))

(event `InputAction|Sprint`
  (params (Key :type "Key Structure" :default "AnyKey"))
  ;[1 1 1] 奔跑
  ;;[1 1 1] 按键持续奔跑
  (:`Pressed`
    (set `self.IsSprint` true)
    (message `/Game/Blueprints/Character/FPSBPI.ToggelSprint` (`self.K2_GetPawn`) (`self.IsSprint`) :!label _label))
  (:`Released`
    (set `self.IsSprint` false)
    (goto _label)))

(event `InputAction|Crouch`
  (params (Key :type "Key Structure" :default "AnyKey"))
  ;[1 1 1] 两种实现方式(cast to会限制转换为固定类型不利于多类型的角色如：AICharacter,TPSCharacter)
  ;;[1 1 1] 持续按键保持蹲伏
  (:`Pressed`
    (set `self.IsCrouched` true)
    (message `/Game/Blueprints/Character/FPSBPI.ToggleCrouch` (`self.K2_GetPawn`) (`self.IsCrouched`) :!label _label_2))
  (:`Released`
    (set `self.IsCrouched` false)
    (goto _label_2)))

(event `InputAction|Jump`
  (params (Key :type "Key Structure" :default "AnyKey"))
  (:`Pressed`
    (message `/Game/Blueprints/Character/FPSBPI.ToggleJump` (`self.K2_GetPawn`))))

(event `InputAction|Fire`
  (params (Key :type "Key Structure" :default "AnyKey"))
  ;[1 1 1] 连续开火
  (:`Pressed`
    (`|ExecutionSequence`
      (:`then_0`
        (goto _label_3 :!via `Open`))
      (:`then_1`
        (`/Engine/EditorBlueprintResources/StandardMacros.Gate` true :!label _label_3
          (:`Exit`
            (`|ExecutionSequence`
              (:`then_0`
                (message `/Game/Blueprints/Character/FPSBPI.HandleFire` (`self.K2_GetPawn`)))
              (:`then_1`
                (`KismetSystemLibrary.RetriggerableDelay` 0.2)
                (goto _label_3))))))))
  (:`Released`
    (goto _label_3 :!via `Close`)))

(event `InputAxis|Turn`
  (params (AxisValue :type "Float (single-precision)"))
  (`self.AddYawInput` AxisValue))

(event `InputAxis|LookUp`
  (params (AxisValue :type "Float (single-precision)"))
  (`self.AddPitchInput` AxisValue))

(event `InputAxis|MoveForward`
  (params (AxisValue :type "Float (single-precision)"))
  (bind (_returnvalue_roll _returnvalue_pitch _returnvalue_yaw) (`KismetMathLibrary.BreakRotator` (`self.GetControlRotation`)))
  ;[1 1 1] 方向移动的另一种实现，低头抬头时w，s可移动
  (`Pawn.AddMovementInput` (`self.K2_GetPawn`) (`KismetMathLibrary.GetForwardVector` (`KismetMathLibrary.MakeRotator` 0.0 0.0 _returnvalue_yaw)) AxisValue false))

(event `InputAxis|MoveRight`
  (params (AxisValue :type "Float (single-precision)"))
  ;[1 1 1] 方向移动的另一种实现，低头抬头时w，s可移动
  (`Pawn.AddMovementInput` (`self.K2_GetPawn`) (`KismetMathLibrary.GetRightVector` (`KismetMathLibrary.MakeRotator` 0.0 0.0 (.yaw (`self.GetControlRotation`)))) AxisValue false))

(fn `CreateScoreHUD`
  (bind _returnvalue (`|CreateWidget` "/Game/UI/ScoreHUD.ScoreHUD_C"))
  (bind _output_get (set `self.ScoreHUD` _returnvalue))
  (`UserWidget.AddToViewport` _output_get 0))

(fn `GetScore`
  (returns (Score :type Integer))
  ;[1 1 1] GameOverHUD中调用
  (return (`self.PlayerScore`)))

(fn `ScoreUpdate`
  (params (ScorePoint :type Integer))
  (bind _output_get (set `self.PlayerScore` (+ ScorePoint (`self.PlayerScore`))))
  (`/Game/UI/ScoreHUD.ScoreDisplay` (`self.ScoreHUD`) _output_get))

(fn `StaminaUpdate`
  (params (Stamina :type Integer))
  (`/Game/UI/ScoreHUD.StaminaDisplay` (`self.ScoreHUD`) Stamina))

(fn `UserConstructionScript`)